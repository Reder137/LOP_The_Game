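; Player hero Character Blueprint that handles basic movement, mouse look and jumping.
; Mouse and movement axes are each gated by boolean flags, with movement along the actor's forward and right vectors scaled by PlayerMaxSpeed.
; Space bar triggers Jump directly through a key event.
; A component hit event prints a debug string and applies a zero impulse, so it has no physical effect.
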(event `InputAxis|Mouse X`
  (params (AxisValue :type "Float (single-precision)"))
  (if (`self.IsMouseInput`)
    (`self.AddControllerYawInput` AxisValue)))

(event `self.Sex.OnComponentHit`
  (params (HitComponent :type "PrimitiveComponent Object Reference") (OtherActor :type "Actor Object Reference") (OtherComp :type "PrimitiveComponent Object Reference") (NormalImpulse :type "Vector Structure") (Hit :type "HitResult Structure (by ref)"))
  (`KismetSystemLibrary.PrintString` "HIT!!!!!")
  (`CharacterMovementComponent.AddImpulse` (`self.CharacterMovement`) (0.0 0.0 0.0) false))

(event `InputAxis|MoveForward `
  (params (AxisValue :type "Float (single-precision)"))
  ;[1 1 1] Base movment
  (if (`self.IsMoveForward`)
    (`self.AddMovementInput` (`self.GetActorForwardVector`) (* AxisValue (`self.PlayerMaxSpeed`)))))

(event `InputAxis|Mouse Y`
  (params (AxisValue :type "Float (single-precision)"))
  (if (`self.IsMouseInput`)
    (`self.AddControllerPitchInput` AxisValue)))

(event `InputAxis|MoveRight`
  (params (AxisValue :type "Float (single-precision)"))
  ;[1 1 1] Base movment
  (if (`self.IsMoveRight`)
    (`self.AddMovementInput` (`self.GetActorRightVector`) (* AxisValue (`self.PlayerMaxSpeed`)))))

(event `Key|SpaceBar`
  (params (Key :type "Key Structure"))
  (:`Pressed`
    (`self.Jump`)))

(fn `UserConstructionScript`)